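; Solitaire-style card column that holds an offset stack of cards and tracks their total weight.
; Updates scan from the last card, glowing pickable alternating-colour, consecutive descending runs, and recalculate the controller's differential when losing is enabled.
; Drops require an empty column or a lower, opposite-colour card.
; Grabbing attaches following cards to the grabbed one, while text previews modifier-scaled weight leaving or entering columns.
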(event EventBeginPlay
  (Rendering|SetVisibility (Variables|Default|GettextBox) false false)
  (bind _asbp_card_game_controller (Utilities|Casting|CastToBP_cardGameController (Game|GetPlayerController 0)))
  (Variables|Default|SetPlayer%20Controller _asbp_card_game_controller))

(event Collision|EventActorBeginOverlap
  (params (OtherActor :type Actor%20Object%20Reference)))

(event EventTick
  (params (DeltaSeconds :type Float%20%28single-precision%29)))

(fn ConstructionScript)

(fn UpdateValue
  (bind _cardsheld (Variables|Default|GetCardsHeld))
  (Variables|Default|SetWeight 0.0)
  (bind (_arrayindex _arrayelement) (Utilities|Array|ReverseforEachLoop _cardsheld) ; Start from last card Held
    (:LoopBody
      (bind _output_get (LocalVariables|SetCardChecked _arrayelement))
      (Variables|Default|SetWeight (+ (Variables|Default|GetWeight) (Variables|/Game/Blueprint/BP_Card.BP_Card_C|GetCardWeight _output_get)))
      ;[0.15 0.15 0.15 0.5] Check what cards are Pickable
      (bind _output_get_2 (LocalVariables|SetLastCardChecked (Utilities|Array|Get(acopy) _cardsheld (+ _arrayindex 1))))
      (if (Utilities|IsValid _output_get_2)
        (Variables|/Game/Blueprint/BP_Card.BP_Card_C|SetCanBePicked (LocalVariables|GetCardChecked) (and (== (Math|Conversions|ToInteger(Byte) (.cardvalue (Variables|/Game/Blueprint/BP_Card.BP_Card_C|GetData (LocalVariables|GetLastCardChecked)))) (- (Math|Conversions|ToInteger(Byte) (.cardvalue (Variables|/Game/Blueprint/BP_Card.BP_Card_C|GetData (LocalVariables|GetCardChecked)))) 1)) (and (!= (Variables|/Game/Blueprint/BP_Card.BP_Card_C|GetIsRed (LocalVariables|GetCardChecked)) (Variables|/Game/Blueprint/BP_Card.BP_Card_C|GetIsRed (LocalVariables|GetLastCardChecked))) (Variables|/Game/Blueprint/BP_Card.BP_Card_C|GetCanBePicked (LocalVariables|GetLastCardChecked)))))
        (else
          (Variables|/Game/Blueprint/BP_Card.BP_Card_C|SetCanBePicked (LocalVariables|GetCardChecked) true)))
      (Rendering|SetVisibility (Variables|/Game/Blueprint/BP_Card.BP_Card_C|GetGlow (LocalVariables|GetCardChecked)) (Variables|/Game/Blueprint/BP_Card.BP_Card_C|GetCanBePicked (LocalVariables|GetCardChecked)) false))
    (:Completed
      (if (Variables|/Game/Blueprint/BP_cardGameController.BP_cardGameController_C|GetCanLose (Variables|Default|GetPlayer%20Controller))
        (Default|CalculateDifferrentiel (Variables|Default|GetPlayer%20Controller))))))

(fn AddCardstoSelf
  (params (NewCard :type Array%20of%20BP%20Card%20Object%20References))
  (bind _cardsheld (Variables|Default|GetCardsHeld))
  (bind _returnvalue (Utilities|Array|LastIndex _cardsheld))
  (bind _output (Utilities|Array|Get(acopy) _cardsheld _returnvalue))
  (for _array_element NewCard
    (bind _output_get (LocalVariables|SetcardBuffer _array_element))
    (if (Utilities|IsValid _output)
      ;[0.15 0.15 0.15 0.5] IF/ELSE
      (Transformation|SetActorLocation _output_get (+ (.location (Transformation|GetActorTransform _output)) (Variables|Default|GetOffSet)) false false)
      (else
        (Transformation|SetActorLocation _output_get (+ (Transformation|GetActorLocation) "0.000000,0.000000,2.000000") false false)))
    (Utilities|Array|AddUnique (Variables|Default|GetCardsHeld) (LocalVariables|GetcardBuffer))
    (Variables|/Game/Blueprint/BP_Card.BP_Card_C|SetStartingColumn (LocalVariables|GetcardBuffer) self))
  (CallFunction|UpdateValue))

(fn CanDrop
  (params (NewCard :type BP%20Card%20Object%20Reference))
  (bind _cardsheld (Variables|Default|GetCardsHeld))
  (bind _returnvalue (Utilities|Array|LastIndex _cardsheld))
  (bind _output (Utilities|Array|Get(acopy) _cardsheld _returnvalue))
  (if (!= (Utilities|Array|Length _cardsheld) 0)
    (return (and (< (Math|Conversions|ToInteger(Byte) (.cardvalue (Variables|/Game/Blueprint/BP_Card.BP_Card_C|GetData NewCard))) (Math|Conversions|ToInteger(Byte) (.cardvalue (Variables|/Game/Blueprint/BP_Card.BP_Card_C|GetData _output)))) (!= (Variables|/Game/Blueprint/BP_Card.BP_Card_C|GetIsRed NewCard) (Variables|/Game/Blueprint/BP_Card.BP_Card_C|GetIsRed _output))))
    (else
      (return true))))

(fn RemoveCardsfromSelf
  (params (NewParam :type BP%20Card%20Object%20Reference))
  (for _array_element (Variables|/Game/Blueprint/BP_cardGameController.BP_cardGameController_C|GetGrabbedPile (Variables|Default|GetPlayer%20Controller))
    (Utilities|Array|RemoveItem (Variables|Default|GetCardsHeld) _array_element))
  (if (Utilities|IsValid NewParam)
    (CallFunction|UpdateValue)))

(fn CreateCardPile
  (params (CardGrabbed :type BP%20Card%20Object%20Reference))
  (bind _textbox (Variables|Default|GettextBox))
  (bind _player_controller (Variables|Default|GetPlayer%20Controller))
  (for _array_element (Variables|Default|GetCardsHeld)
    (if (or (LocalVariables|GetStartPile) (== _array_element CardGrabbed))
      (if (LocalVariables|GetStartPile)
        (Transformation|AttachActorToActor _array_element (Variables|/Game/Blueprint/BP_cardGameController.BP_cardGameController_C|GetGrabbedCard _player_controller) "None" "KeepWorld" "KeepWorld" "KeepWorld" true))
      (LocalVariables|SetStartPile true)
      (Utilities|Array|AddUnique (Variables|/Game/Blueprint/BP_cardGameController.BP_cardGameController_C|GetGrabbedPile _player_controller) _array_element)
      (LocalVariables|SetBufferweight (+ (Variables|/Game/Blueprint/BP_Card.BP_Card_C|GetCardWeight _array_element) (LocalVariables|GetBufferweight)))))
  (if (Utilities|IsValid (Variables|Default|GettextBox))
    (Rendering|Components|TextRender|SetText _textbox (Utilities|Text|ToText(String) (Utilities|String|Append "- " (Utilities|String|ToString(Text) (Utilities|Text|ToText(Float) (* (Variables|Default|GetModifier) (LocalVariables|GetBufferWeight)) "HalfToEven")))))
    (Rendering|Components|TextRender|SetTextRenderColor _textbox (Math|Color|MakeColor 0 0 100 0))
    (Rendering|SetVisibility _textbox true false)))

(fn UpdateText
  (bind _player_controller (Variables|Default|GetPlayer%20Controller))
  (bind _textbox (Variables|Default|GettextBox))
  (for _array_element (Variables|/Game/Blueprint/BP_Deck.BP_Deck_C|GetColumnsDeck (Variables|/Game/Blueprint/BP_cardGameController.BP_cardGameController_C|GetCardManager (Variables|Default|GetPlayer%20Controller)))
    (if (!= _array_element (Variables|/Game/Blueprint/BP_Card.BP_Card_C|GetStartingColumn (Variables|/Game/Blueprint/BP_cardGameController.BP_cardGameController_C|GetGrabbedCard _player_controller)))
      (Rendering|SetVisibility (Variables|BP_Column_C|GettextBox _array_element) false false)))
  (for _array_element_2 (Variables|/Game/Blueprint/BP_cardGameController.BP_cardGameController_C|GetGrabbedPile _player_controller)
    (LocalVariables|SetBufferWeight (+ (LocalVariables|GetBufferWeight) (Variables|/Game/Blueprint/BP_Card.BP_Card_C|GetCardWeight _array_element_2))))
  (if (!= self (Variables|/Game/Blueprint/BP_Card.BP_Card_C|GetStartingColumn (Variables|/Game/Blueprint/BP_cardGameController.BP_cardGameController_C|GetGrabbedCard (Variables|Default|GetPlayer%20Controller))))
    (Rendering|Components|TextRender|SetText (Variables|Default|GettextBox) (Utilities|Text|ToText(String) (Utilities|String|Append "+ " (Utilities|String|ToString(Text) (Utilities|Text|ToText(Float) (* (LocalVariables|GetBufferWeight) (Variables|Default|GetModifier)) "HalfToEven")))))
    (Rendering|Components|TextRender|SetTextRenderColor _textbox (Math|Color|MakeColor 100 0 0 0))
    (Rendering|SetVisibility _textbox true false)))