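; Deck actor for a column-based card game that deals the cards and tracks the win condition.
; After a short BeginPlay delay, it builds shuffled color/value pairs from a difficulty-specific enum, then spawns them as offset BP_Card rows across ColumnsDeck, setting column modifiers.
; It registers with BP_cardGameController, which calculates the differential.
; CheckWinCon decrements the in-play count to trigger Win, while ReShuffle redistributes existing cards across the columns.
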(event EventBeginPlay
  ;[0.15 0.15 0.15 0.5] wait for player to be created
  (Utilities|FlowControl|Delay 0.2)
  (bind _asbp_game_instance (Utilities|Casting|CastToBP_GameInstance (Game|GetGameInstance)))
  (Variables|Default|SetDifficultySwitch (Variables|/Game/Blueprint/BP_GameInstance.BP_GameInstance_C|GetDifficulty _asbp_game_instance))
  (CallFunction|SpawnCards)
  (bind _asbp_card_game_controller (Utilities|Casting|CastToBP_cardGameController (Game|GetPlayerController 0)))
  (bind _output_get (Variables|Default|SetPlayer _asbp_card_game_controller))
  (Variables|/Game/Blueprint/BP_cardGameController.BP_cardGameController_C|SetCardManager _output_get self)
  (Variables|/Game/Blueprint/BP_cardGameController.BP_cardGameController_C|SetColumns _output_get (Variables|Default|GetColumnsDeck))
  (Default|CalculateDifferrentiel _output_get)
  (Variables|/Game/Blueprint/BP_cardGameController.BP_cardGameController_C|SetCanLose _output_get true))

(event Collision|EventActorBeginOverlap
  (params (OtherActor :type Actor%20Object%20Reference)))

(event EventTick
  (params (DeltaSeconds :type Float%20%28single-precision%29)))

(fn ConstructionScript)

(fn SpawnCards
  (bind _carddata (LocalVariables|GetcardData))
  (bind _enumvalue (|ForEachEN_CardColor)
    (:LoopBody
      (switch int (Variables|Default|GetDifficultySwitch)
        (:0
          (Variables|Default|SetEnumEntries_ (|GetNumEnumEntries))
          (bind _enumvalue_2 (|ForEachEN_CardValueEasy)
            (:LoopBody
              (LocalVariables|SetEnumBuffer (Utilities|Enum|ByteToEnumEN_CardValueHard (Math|Conversions|ToByte(Integer) (Math|Conversions|ToInteger(Byte) _enumvalue_2)))))))
        (:1
          (Variables|Default|SetEnumEntries_ (|GetNumEnumEntries))
          (bind _enumvalue_3 (|ForEachEN_CardValue)
            (:LoopBody
              (LocalVariables|SetEnumBuffer (Utilities|Enum|ByteToEnumEN_CardValueHard (Math|Conversions|ToByte(Integer) (Math|Conversions|ToInteger(Byte) _enumvalue_3)))))))
        (:2
          (Variables|Default|SetEnumEntries_ (|GetNumEnumEntries))
          (bind _enumvalue_4 (|ForEachEN_CardValueHard)
            (:LoopBody
              (LocalVariables|SetEnumBuffer (Utilities|Enum|ByteToEnumEN_CardValueHard (Math|Conversions|ToByte(Integer) (Math|Conversions|ToInteger(Byte) _enumvalue_4))))))))
      (Utilities|Array|AddUnique (LocalVariables|GetcardData) (Utilities|Struct|MakeSt_CardData (LocalVariables|GetEnumBuffer) _enumvalue)))
    (:then
      (LocalVariables|SetColumnIndex 0)
      (Utilities|Array|Shuffle _carddata)
      (for (_array_element _array_index) _carddata
        (LocalVariables|SetArrayIndexVR _array_index)
        (bind _returnvalue (Game|SpawnActorfromClass "/Game/Blueprint/BP_Card.BP_Card_C" (Math|Transform|MakeTransform (+ (Variables|Default|GetCardOffset) (.location (Transformation|GetActorTransform (Utilities|Array|Get(acopy) (Variables|Default|GetColumnsDeck) (LocalVariables|GetColumnIndex))))) (.rotation (Transformation|GetActorTransform (Utilities|Array|Get(acopy) (Variables|Default|GetColumnsDeck) (LocalVariables|GetColumnIndex)))) "1.000000,1.000000,1.000000") "Undefined" "MultiplyWithRoot" 0 _array_element 0))
        (Variables|/Game/Blueprint/BP_Card.BP_Card_C|SetStartingColumn _returnvalue (Utilities|Array|Get(acopy) (Variables|Default|GetColumnsDeck) (LocalVariables|GetColumnIndex)))
        (Utilities|Array|AddUnique (Variables|/Game/Blueprint/BP_Column.BP_Column_C|GetCardsHeld (Utilities|Array|Get(acopy) (Variables|Default|GetColumnsDeck) (LocalVariables|GetColumnIndex))) _returnvalue)
        (if (== (Math|Integer|%(Integer) (+ (LocalVariables|GetArrayIndexVR) 1) (Variables|Default|GetEnumEntries_)) 0)
          (if (or (== (LocalVariables|GetColumnIndex) 0) (== (LocalVariables|GetColumnIndex) 3))
            ;[0.15 0.15 0.15 0.5] IF/ELSE
            (Variables|/Game/Blueprint/BP_Column.BP_Column_C|SetModifier (Utilities|Array|Get(acopy) (Variables|Default|GetColumnsDeck) (LocalVariables|GetColumnIndex)) 1.0)
            (else
              (Variables|/Game/Blueprint/BP_Column.BP_Column_C|SetModifier (Utilities|Array|Get(acopy) (Variables|Default|GetColumnsDeck) (LocalVariables|GetColumnIndex)) 0.5)))
          (Default|UpdateValue (Utilities|Array|Get(acopy) (Variables|Default|GetColumnsDeck) (LocalVariables|GetColumnIndex)))
          (LocalVariables|SetColumnIndex (+ 1 (LocalVariables|GetColumnIndex)))
          (Variables|Default|SetCardOffset "0, 0, 0")
          (else
            (Variables|Default|SetCardOffset (+ (Variables|Default|GetCardOffset) "40.000000,0.000000,1.000000")))))
      (Variables|Default|SetNbCardInPlay (Utilities|Array|Length _carddata)))))

(fn CheckWinCon
  (bind _result (Math|Integer|DecrementInt (Variables|Default|GetNbCardInPlay))
    (:%20%20
      (if (<= _result 2)
        (Default|Win (Variables|Default|GetPlayer))))))

(fn ReShuffle
  (for _array_element (Variables|Default|GetColumnsDeck)
    (Utilities|Array|Clear (Variables|/Game/Blueprint/BP_Column.BP_Column_C|GetCardsHeld _array_element)))
  (bind _outactors (Actor|GetAllActorsOfClass "/Game/Blueprint/BP_Card.BP_Card_C"))
  (bind _output_get (LocalVariables|SetAllCards _outactors))
  (Utilities|Array|Shuffle _output_get)
  (for (_array_element_2 _array_index) _output_get
    (LocalVariables|SetbufferCard _array_element_2)
    (LocalVariables|SetIndexArray _array_index)
    (Transformation|SetActorLocation _array_element_2 (+ (Variables|Default|GetCardOffset) (.location (Transformation|GetActorTransform (Utilities|Array|Get(acopy) (Variables|Default|GetColumnsDeck) (LocalVariables|GetColumnIndex))))) false false)
    (Variables|/Game/Blueprint/BP_Card.BP_Card_C|SetStartingColumn (LocalVariables|GetbufferCard) (Utilities|Array|Get(acopy) (Variables|Default|GetColumnsDeck) (LocalVariables|GetColumnIndex)))
    (Utilities|Array|AddUnique (Variables|/Game/Blueprint/BP_Column.BP_Column_C|GetCardsHeld (Utilities|Array|Get(acopy) (Variables|Default|GetColumnsDeck) (LocalVariables|GetColumnIndex))) (LocalVariables|GetbufferCard))
    (if (== (Math|Integer|%(Integer) (+ (LocalVariables|GetIndexArray) 1) (Variables|Default|GetEnumEntries_)) 0)
      (Default|UpdateValue (Utilities|Array|Get(acopy) (Variables|Default|GetColumnsDeck) (LocalVariables|GetColumnIndex)))
      (LocalVariables|SetColumnIndex (+ 1 (LocalVariables|GetColumnIndex)))
      (Variables|Default|SetCardOffset "0, 0, 0")
      (else
        (Variables|Default|SetCardOffset (+ (Variables|Default|GetCardOffset) "40.000000,0.000000,1.000000")))))
  (Variables|Default|SetNbCardInPlay (Utilities|Array|Length _output_get))
  (Default|CalculateDifferrentiel (Variables|Default|GetPlayer)))