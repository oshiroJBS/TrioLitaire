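; Free-space slot for a card game, a child card-holder Blueprint that can hold a single card.
; BeginPlay removes its TextBox and caches the card game controller, which CanDrop checks to accept only a one-card grabbed pile into an empty slot.
; UpdateText hides the text on every column except the grabbed card's starting one.
; Adding cards defers to the parent, and UpdateValue is empty.
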(event EventBeginPlay
  (Components|DestroyComponent (Variables|Default|GettextBox))
  (bind _asbp_card_game_controller (Utilities|Casting|CastToBP_cardGameController (Game|GetPlayerController 0)))
  (Variables|Default|SetPlayer%20Controller _asbp_card_game_controller))

(event Collision|EventActorBeginOverlap
  (params (OtherActor :type Actor%20Object%20Reference)))

(event EventTick
  (params (DeltaSeconds :type Float%20%28single-precision%29)))

(fn ConstructionScript)

(fn CanDrop
  (params (NewCard :type BP%20Card%20Object%20Reference))
  (return (and (== (Utilities|Array|Length (Variables|Default|GetCardsHeld)) 0) (== 1 (Utilities|Array|Length (Variables|/Game/Blueprint/BP_cardGameController.BP_cardGameController_C|GetGrabbedPile (Variables|Default|GetPlayer%20Controller)))))))

(fn UpdateValue)

(fn UpdateText
  (for _array_element (Variables|/Game/Blueprint/BP_Deck.BP_Deck_C|GetColumnsDeck (Variables|/Game/Blueprint/BP_cardGameController.BP_cardGameController_C|GetCardManager (Variables|Default|GetPlayer%20Controller)))
    (if (!= _array_element (Variables|/Game/Blueprint/BP_Card.BP_Card_C|GetStartingColumn (Variables|/Game/Blueprint/BP_cardGameController.BP_cardGameController_C|GetGrabbedCard (Variables|Default|GetPlayer%20Controller))))
      (Rendering|SetVisibility (Variables|/Game/Blueprint/BP_Column.BP_Column_C|GettextBox _array_element) false false))))

(fn AddCardstoSelf
  (params (NewCard :type Array%20of%20BP%20Card%20Object%20References))
  (|CallParentFunction NewCard)
  (return))