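; BP_EndTiles is a foundation-style end tile in a solitaire-like card game, where cards build upward toward the win condition.
; CanDrop takes only a single grabbed card: value zero on an empty tile, otherwise the next value in the top card's color.
; AddCardsToSelf extends the parent's version by snapping cards to the tile in X/Y, making them unpickable, and calling the Deck's win check for each.
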(event EventBeginPlay
  (Components|DestroyComponent (Variables|Default|GettextBox))
  (bind _asbp_card_game_controller (Utilities|Casting|CastToBP_cardGameController (Game|GetPlayerController 0)))
  (Variables|Default|SetPlayer%20Controller _asbp_card_game_controller)
  (bind _returnvalue (Actor|GetActorOfClass "/Game/Blueprint/BP_Deck.BP_Deck_C"))
  (Variables|Default|SetDeck _returnvalue))

(event Collision|EventActorBeginOverlap
  (params (OtherActor :type Actor%20Object%20Reference)))

(event EventTick
  (params (DeltaSeconds :type Float%20%28single-precision%29)))

(fn ConstructionScript)

(fn CanDrop
  (params (NewCard :type BP%20Card%20Object%20Reference))
  (bind _player_controller (Variables|Default|GetPlayer%20Controller))
  (bind _cardsheld (Variables|Default|GetCardsHeld))
  (bind _returnvalue (Utilities|Array|LastIndex _cardsheld))
  (bind _grabbedpile (Variables|/Game/Blueprint/BP_cardGameController.BP_cardGameController_C|GetGrabbedPile _player_controller))
  (bind _data (Variables|/Game/Blueprint/BP_Card.BP_Card_C|GetData NewCard))
  (bind _output (Utilities|Array|Get(acopy) _cardsheld _returnvalue))
  (bind _data_2 (Variables|/Game/Blueprint/BP_Card.BP_Card_C|GetData _output))
  (if (== 1 (Utilities|Array|Length (Variables|/Game/Blueprint/BP_cardGameController.BP_cardGameController_C|GetGrabbedPile (Variables|Default|GetPlayer%20Controller))))
    (if (== (Utilities|Array|Length (Variables|Default|GetCardsHeld)) 0)
      (LocalVariables|Setbuffer (== (Math|Conversions|ToInteger(Byte) (.cardvalue (Variables|/Game/Blueprint/BP_Card.BP_Card_C|GetData (Utilities|Array|Get(acopy) _grabbedpile (Utilities|Array|LastIndex _grabbedpile))))) 0))
      (else
        (LocalVariables|Setbuffer (and (== (Math|Conversions|ToInteger(Byte) (.cardvalue _data)) (+ (Math|Conversions|ToInteger(Byte) (.cardvalue _data_2)) 1)) (== (Math|Conversions|ToInteger(Byte) (.cardcolor _data)) (Math|Conversions|ToInteger(Byte) (.cardcolor _data_2)))))))
    (return (LocalVariables|Getbuffer))))

(fn AddCardstoSelf
  (params (NewCard :type Array%20of%20BP%20Card%20Object%20References))
  (bind _self self)
  (bind _returnvalue (Transformation|GetActorLocation _self))
  (|CallParentFunction NewCard)
  (for _array_element NewCard
    (Transformation|SetActorLocation _array_element (Math|Vector|MakeVector (.x _returnvalue) (.y _returnvalue) (.z (Transformation|GetActorLocation _array_element))) false false)
    (Variables|/Game/Blueprint/BP_Card.BP_Card_C|SetCanBePicked _array_element false)
    (Default|CheckWinCon (Variables|Default|GetDeck)))
  (return))

(fn UpdateValue
  (|CallParentFunction))