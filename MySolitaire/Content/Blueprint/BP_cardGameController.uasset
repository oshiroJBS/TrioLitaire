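; Controller for a column-based card game with a weight-balance rule, handling mouse card dragging, the HUD and win/lose screens.
; Grabbed cards follow the deprojected cursor at a floating height, then move to the new column on release or snap back if disallowed.
; CalculateDifferrentiel compares left and right column weights, outer columns counting double, and updates the HUD.
; Too much imbalance triggers a reshuffle, or a loss once CanLose is set.
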(event Custom|GrabCard
  (params (Card :type BP%20Card%20Object%20Reference) (StartingPosition :type Vector))
  (if (Utilities|IsValid (Variables|Default|GetGrabbedCard))
    (Development|PrintText "ALREADY GRABBED A CARD")
    (else
      (bind _output_get (Variables|Default|SetGrabbedCard Card))
      (Variables|Default|SetStartingPositionOfCard StartingPosition)
      (Variables|Default|SetGrabOffset (- (Transformation|GetActorLocation _output_get) (.WorldLocation (Game|Player|ConvertMouseLocationToWorldSpace))))
      (Default|CreateCardPile (Variables|/Game/Blueprint/BP_Card.BP_Card_C|GetStartingColumn (Variables|Default|GetGrabbedCard)) (Variables|Default|GetGrabbedCard))
      (Variables|/Game/Blueprint/BP_Card.BP_Card_C|SetIsPicked (Variables|Default|GetGrabbedCard) true))))

(event Custom|RealeseCard
  (bind _grabbedpile (Variables|Default|GetGrabbedPile))
  (if (Utilities|IsValid (Variables|Default|GetGrabbedCard))
    (if (Utilities|IsValid (Variables|/Game/Blueprint/BP_Card.BP_Card_C|GetNewColumn (Variables|Default|GetGrabbedCard)))
      (bind _canbedroppedhere (Default|CanDrop (Variables|/Game/Blueprint/BP_Card.BP_Card_C|GetNewColumn (Variables|Default|GetGrabbedCard)) (Variables|Default|GetGrabbedCard)))
      (if _canbedroppedhere
        (Default|RemoveCardsfromSelf (Variables|/Game/Blueprint/BP_Card.BP_Card_C|GetStartingColumn (Variables|Default|GetGrabbedCard)) (Variables|Default|GetGrabbedCard))
        (Default|AddCardstoSelf (Variables|/Game/Blueprint/BP_Card.BP_Card_C|GetNewColumn (Variables|Default|GetGrabbedCard)) (Variables|Default|GetGrabbedPile))
        (else
          (Transformation|SetActorLocation (Variables|Default|GetGrabbedCard) (Variables|Default|GetStartingPositionOfCard) false true :!label _label)))
      (else
        (goto _label)))
    (Variables|Default|SetGrabbedCard 0)
    (for _array_element _grabbedpile
      (Transformation|DetachFromActor _array_element "KeepWorld" "KeepWorld" "KeepWorld"))
    (Utilities|Array|Clear _grabbedpile)
    (for _array_element_2 (Variables|/Game/Blueprint/BP_Deck.BP_Deck_C|GetColumnsDeck (Variables|Default|GetCardManager))
      (Rendering|SetVisibility (Variables|/Game/Blueprint/BP_Column.BP_Column_C|GettextBox _array_element_2) false false))))

(event EventBeginPlay
  (bind _returnvalue (UserInterface|CreateWidget "/Game/HUD/WD_HUD.WD_HUD_C"))
  (bind _output_get (Variables|Default|SetPlayerHUD _returnvalue))
  (UserInterface|Viewport|AddtoViewport _output_get 0))

(event EventTick
  (params (DeltaSeconds :type Float%20%28single-precision%29))
  (bind _worldlocation (Game|Player|ConvertMouseLocationToWorldSpace))
  (bind _grabbedcard (Variables|Default|GetGrabbedCard))
  (bind _graboffset (Variables|Default|GetGrabOffset))
  (bind _returnvalue (+ _worldlocation _graboffset))
  (Utilities|IsValid _grabbedcard
    (:Is%20Valid
      (Transformation|SetActorLocation _grabbedcard (Math|Vector|MakeVector (.x _returnvalue) (.y _returnvalue) (Variables|Default|GetfloatingZ)) false false))))

(fn ConstructionScript
  (Variables|Default|SetCanLose false))

(fn CalculateDifferrentiel
  (for (_array_element _array_index) (Variables|Default|GetColumns)
    (LocalVariables|SetBufferColumn _array_element)
    (switch int _array_index
      (:0
        ;[0.15 0.15 0.15 0.5] Calculate Weight
        (LocalVariables|SetRightWeight (+ (Variables|/Game/Blueprint/BP_Column.BP_Column_C|GetWeight (LocalVariables|GetBufferColumn)) (LocalVariables|GetRightWeight))))
      (:1
        (LocalVariables|SetRightWeight (+ (LocalVariables|GetRightWeight) (/ (Variables|/Game/Blueprint/BP_Column.BP_Column_C|GetWeight (LocalVariables|GetBufferColumn)) 2.0))))
      (:2
        (LocalVariables|SetLeftWeight (+ (LocalVariables|GetLeftWeight) (/ (Variables|/Game/Blueprint/BP_Column.BP_Column_C|GetWeight (LocalVariables|GetBufferColumn)) 2.0))))
      (:3
        (LocalVariables|SetLeftWeight (+ (LocalVariables|GetLeftWeight) (Variables|/Game/Blueprint/BP_Column.BP_Column_C|GetWeight (LocalVariables|GetBufferColumn)))))))
  (if (> (LocalVariables|GetRightWeight) (LocalVariables|GetLeftWeight))
    ;[0.15 0.15 0.15 0.5] IF/ELSE
    (LocalVariables|Setdifferentiel (/ (LocalVariables|GetLeftWeight) (LocalVariables|GetRightWeight)))
    (else
      (LocalVariables|Setdifferentiel (/ (LocalVariables|GetRightWeight) (LocalVariables|GetLeftWeight)))))
  (Default|SetWeightValue (Variables|Default|GetPlayerHUD) (LocalVariables|GetLeftWeight) (LocalVariables|GetRightWeight) (LocalVariables|Getdifferentiel))
  (if (Variables|Default|GetCanLose)
    (if (< (LocalVariables|Getdifferentiel) 0.5)
      (CallFunction|Lose))
    (elif (< (LocalVariables|Getdifferentiel) 0.75)
      (Default|ReShuffle (Variables|Default|GetCardManager)))))

(fn CreateHud
  (bind _returnvalue (UserInterface|CreateWidget "/Game/HUD/WD_HUD.WD_HUD_C"))
  (bind _output_get (Variables|Default|SetPlayerHUD _returnvalue))
  (UserInterface|Viewport|AddtoViewport _output_get 0))

(fn Lose
  (bind _playerhud (Variables|Default|GetPlayerHUD))
  (Widget|SetVisibility (Variables|/Game/HUD/WD_HUD.WD_HUD_C|GetInGameRestart _playerhud) "Hidden")
  (Widget|SetVisibility (Variables|/Game/HUD/WD_HUD.WD_HUD_C|GetLoseScreen _playerhud) "Visible"))

(fn Win
  (Widget|SetVisibility (Variables|/Game/HUD/WD_HUD.WD_HUD_C|GetWinScreen (Variables|Default|GetPlayerHUD)) "Visible"))