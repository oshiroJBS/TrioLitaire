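; BP_Card is a playing card actor that the player picks up and drags between columns in a card game.
; It pushes its data into a WD_CardFace widget and on BeginPlay derives a red flag and a weight, bounded by the GameInstance difficulty value.
; Click and release delegate grabbing to BP_cardGameController, while overlaps during a pick track the target BP_Column.
; CanDrop always returns false here.
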(event EventBeginPlay
  (bind _data (Variables|Default|GetData))
  (bind _asbp_card_game_controller (Utilities|Casting|CastToBP_cardGameController (Game|GetPlayerController 0)))
  (Variables|Default|SetPlayerController _asbp_card_game_controller)
  (bind _aswd_card_face (Utilities|Casting|CastToWD_CardFace (UserInterface|GetWidget (Variables|Default|GetWidget))))
  (bind _output_get (Variables|Default|SetDataCard _aswd_card_face))
  (Default|SetCardData _output_get (Utilities|Struct|MakeSt_CardData (.cardvalue _data) (.cardcolor _data)))
  (Variables|Default|SetIsRed (or (Utilities|Enum|Equal(Enum) (.cardcolor _data) "NewEnumerator2") (Utilities|Enum|Equal(Enum) (.cardcolor _data) "NewEnumerator3")))
  (bind _asbp_game_instance (Utilities|Casting|CastToBP_GameInstance (Game|GetGameInstance)))
  (for _index (range 0 (- (Variables|/Game/Blueprint/BP_GameInstance.BP_GameInstance_C|GetDifficultyEnumValue _asbp_game_instance) 1))
    (if (== (Math|Conversions|ToInteger(Byte) (.cardvalue (Variables|Default|GetData))) _index)
      (Variables|Default|SetCardWeight (Math|Conversions|ToFloat(Integer) (+ _index 1))))))

(event Collision|EventActorBeginOverlap
  (params (OtherActor :type Actor%20Object%20Reference))
  ;[0.15 0.15 0.15 0.5] Overlap
  (if (Variables|Default|GetIsPicked)
    (bind _asbp_column (Utilities|Casting|CastToBP_Column OtherActor))
    (bind _output_get (Variables|Default|SetNewColumn _asbp_column))
    (Default|UpdateText _output_get)))

(event MouseInput|EventActorOnClicked
  (params (ButtonPressed :type Key%20Structure :default "None"))
  (bind _self self)
  (bind _returnvalue (Transformation|GetActorLocation _self))
  ;[0.15 0.15 0.15 0.5] Click Management
  (if (Variables|Default|GetCanBePicked)
    (Variables|Default|SetStartingPos _returnvalue)
    (if (not (Utilities|IsValid (Variables|/Game/Blueprint/BP_cardGameController.BP_cardGameController_C|GetGrabbedCard (Variables|Default|GetPlayerController))))
      (Default|GrabCard (Variables|Default|GetPlayerController) self _returnvalue))))

(event EventActorOnReleased
  (params (ButtonReleased :type Key%20Structure :default "None"))
  ;[0.15 0.15 0.15 0.5] Click Management
  (Default|RealeseCard (Variables|Default|GetPlayerController)))

(event Collision|EventActorEndOverlap
  (params (OtherActor :type Actor%20Object%20Reference))
  ;[0.15 0.15 0.15 0.5] Overlap
  (if (Variables|Default|GetIsPicked)
    (bind _asbp_column (Utilities|Casting|CastToBP_Column OtherActor))
    (if (== _asbp_column (Variables|Default|GetNewColumn))
      (Variables|Default|SetNewColumn 0))))

(fn ConstructionScript
  (bind _aswd_card_face (Utilities|Casting|CastToWD_CardFace (UserInterface|GetWidget (Variables|Default|GetWidget))))
  (bind _output_get (Variables|Default|SetDataCard _aswd_card_face))
  (Default|SetCardData _output_get (Variables|Default|GetData)))

(fn CanDrop
  (params (cardHeld :type BP%20Card%20Object%20Reference))
  (return false))